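; Hideable locker actor: inside its trigger box, the player presses IA_Hide to get in or out as the door timeline plays.
; Box overlap toggles input and a gate; ToggleHide hides the character, swaps collision with a child hide box, and blends view to the locker.
; While hidden, IA_Look accumulates clamped pitch and yaw, applied to the camera by a self-calling MoveCamera delay loop.
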(event `self.ReceiveBeginPlay`)

(event `EnhancedInput|/Game/Custom_Assets/Locker/IA_Hide`
  (params (ActionValue :type Boolean) (ElapsedSeconds :type "Float (double-precision)") (TriggeredSeconds :type "Float (double-precision)") (InputAction :type "InputAction Object Reference" :default "/Game/Custom_Assets/Locker/IA_Hide.IA_Hide"))
  ;[1 1 1] Getting in and out
  (:`Started`
    (`MovementComponent.StopMovementImmediately` (`Character.CharacterMovement` (`GameplayStatics.GetPlayerCharacter` 0)))
    (`/Engine/EditorBlueprintResources/StandardMacros.Gate` true :!label _label
      (:`Exit`
        (`|ExecutionSequence`
          (:`then_0`
            (`self.ToggleHide`)
            (`self.MoveCamera`)
            (`KismetSystemLibrary.Delay` 0.2)
            (`self.EnableInput` (`GameplayStatics.GetPlayerController` 0) :!label _label_2)
            (goto _label :!via `Open`))
          (:`then_1`
            (bind (_direction _doortrack) (`Timeline|T_OpenCloseDoor` :!via `PlayFromStart`)
              (:`Update`
                (`SceneComponent.K2_SetRelativeRotation` (`self.Locker_Door`) (`KismetMathLibrary.MakeRotator` 0.0 0.0 (`KismetMathLibrary.Lerp` (`self.CloseAngle`) (`self.OpenAngle`) _doortrack)) false false)))))))))

(event `self.Box.OnComponentBeginOverlap`
  (params (OverlappedComponent :type "PrimitiveComponent Object Reference") (OtherActor :type "Actor Object Reference") (OtherComp :type "PrimitiveComponent Object Reference") (OtherBodyIndex :type Integer) (bFromSweep :type Boolean) (SweepResult :type "HitResult Structure (by ref)"))
  ;[1 1 1] Getting in and out
  (bind _asbp_third_person_character (cast `/Game/ThirdPerson/Blueprints/BP_ThirdPersonCharacter` OtherActor))
  (set `self.Char_Ref` _asbp_third_person_character)
  (goto _label_2))

(event `self.Box.OnComponentEndOverlap`
  (params (OverlappedComponent :type "PrimitiveComponent Object Reference") (OtherActor :type "Actor Object Reference") (OtherComp :type "PrimitiveComponent Object Reference") (OtherBodyIndex :type Integer))
  ;[1 1 1] Getting in and out
  (cast `/Game/ThirdPerson/Blueprints/BP_ThirdPersonCharacter` OtherActor)
  (`self.DisableInput` (`GameplayStatics.GetPlayerController` 0))
  (goto _label :!via `Close`))

(event `EnhancedInput|/Game/ThirdPerson/Input/Actions/IA_Look`
  (params (ActionValue :type "Vector2D Structure") (ElapsedSeconds :type "Float (double-precision)") (TriggeredSeconds :type "Float (double-precision)") (InputAction :type "InputAction Object Reference" :default "/Game/ThirdPerson/Input/Actions/IA_Look.IA_Look"))
  ;[1 1 1] Camera Setup
  (:`Triggered`
    (if (`self.IsHiding`)
      ;;[1 1 1] Setup Pitch (Y)
      (bind _output_get (set `self.Pitch` (`KismetMathLibrary.FClamp` (+ (`self.Pitch`) ActionValue_Y) -40.0 20.0))))))

(event `MoveCamera`
  ;[1 1 1] Camera Setup
  (if (`self.IsHiding`)
    (`SceneComponent.K2_SetRelativeRotation` (`self.Camera`) (`KismetMathLibrary.MakeRotator` 0.0 (* (stale `EnhancedInput|/Game/ThirdPerson/Input/Actions/IA_Look` _output_get) -1.0) (stale `EnhancedInput|/Game/ThirdPerson/Input/Actions/IA_Look` _output_get)) false false)
    (`KismetSystemLibrary.Delay` 0.001)
    (`self.MoveCamera`)))

(event `EnhancedInput|/Game/ThirdPerson/Input/Actions/IA_Look`
  (params (ActionValue :type "Vector2D Structure") (ElapsedSeconds :type "Float (double-precision)") (TriggeredSeconds :type "Float (double-precision)") (InputAction :type "InputAction Object Reference" :default "/Game/ThirdPerson/Input/Actions/IA_Look.IA_Look"))
  ;[1 1 1] Camera Setup
  (:`Triggered`
    (if (`self.IsHiding`)
      ;;[1 1 1] Setup Yaw X
      (bind _output_get (set `self.Yaw` (`KismetMathLibrary.FClamp` (+ (`self.Yaw`) ActionValue_X) -60.0 60.0))))))

(fn `ToggleHide`
  (bind _returnvalue (`GameplayStatics.GetPlayerController` 0))
  (bind _camblendtime (`self.CamBlendTime`))
  (bind _char_ref (`self.Char_Ref`))
  (bind _childactor (`ChildActorComponent.ChildActor` (`self.BP_HideBox2`)))
  (if (`self.IsHiding`)
    ;[0.5002 0.5259 1] Sets var- IsHiding on/off based on its state
    (set `self.IsHiding` false)
    (`self.SetActorHiddenInGame` _char_ref false)
    (`self.SetActorEnableCollision` _char_ref true)
    (`self.SetActorEnableCollision` _childactor false)
    (`PlayerController.SetViewTargetWithBlend` _returnvalue _char_ref _camblendtime "VTBlend_Linear" 0.0 false)
    (else
      (set `self.IsHiding` true)
      ;[1 1 1] Hides the player and disables collision
      (`self.SetActorHiddenInGame` _char_ref true)
      (`self.SetActorEnableCollision` _char_ref false)
      ;[1 1 1] Creates a box which hides the player
      (`self.SetActorEnableCollision` _childactor true)
      ;[1 1 1] Changes to locker camera
      (`PlayerController.SetViewTargetWithBlend` _returnvalue self _camblendtime "VTBlend_Linear" 0.0 false))))

(fn `UserConstructionScript`)